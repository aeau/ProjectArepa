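; BP_EnemyFollower is an enemy that chases the TwinStickPawn and kills it on contact.
; PawnSensing starts an AI MoveTo toward the seen TwinStickPawn, and a Sphere overlap calls that pawn's Death.
; LoseHealth removes one Health per call and triggers the enemy's own Death at zero or below, which spawns an explosion effect and sound, then destroys the actor.
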(event OnSeePawn(PawnSensing)
  (params (Pawn :type Pawn%20Object%20Reference))
  (bind _astwin_stick_pawn (Utilities|Casting|CastToTwinStickPawn Pawn))
  (AI|AIMoveTo self "0, 0, 0" _astwin_stick_pawn 5.0 false))

(event OnComponentBeginOverlap(Sphere)
  (params (OverlappedComponent :type Primitive%20Component%20Object%20Reference) (OtherActor :type Actor%20Object%20Reference) (OtherComp :type Primitive%20Component%20Object%20Reference) (OtherBodyIndex :type Integer) (bFromSweep :type Boolean) (SweepResult :type Hit%20Result%20Structure%20%28by%20ref%29))
  (bind _astwin_stick_pawn (Utilities|Casting|CastToTwinStickPawn OtherActor))
  (Default|Death _astwin_stick_pawn))

(event Custom|LoseHealth
  (bind _output_get (Variables|Default|SetHealth (- (Variables|Default|GetHealth) 1)))
  (if (<= _output_get 0)
    (CallFunction|Death)))

(event Custom|Death
  (Effects|SpawnEmitteratLocation "/Game/StarterContent/Particles/P_Explosion.P_Explosion" (Transformation|GetActorLocation))
  (Audio|SpawnSound2D "/Game/Sounds/ExplosionShortCue.ExplosionShortCue")
  (Actor|DestroyActor))

(fn ConstructionScript)