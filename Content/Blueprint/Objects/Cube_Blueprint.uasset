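; Destructible cube actor that loses health when hit and explodes when that health runs out.
; Its TakeDamage function subtracts DamageTaken from Health, then plays an explosion sound and particle effect and destroys the actor at zero or below.
; Non-lethal hits play a laser sound and a light explosion effect at the cube's location.
; The event graph and construction script are empty, so all behavior lives in that function.
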(event EventBeginPlay)

(event Collision|EventActorBeginOverlap
  (params (OtherActor :type Actor%20Object%20Reference)))

(event EventTick
  (params (DeltaSeconds :type Float%20%28single-precision%29)))

(fn ConstructionScript)

(fn TakeDamage
  (bind _returnvalue (Transformation|GetActorLocation))
  (bind _output_get (Variables|Default|SetHealth (- (Variables|Default|GetHealth) (Variables|Default|GetDamageTaken))))
  (if (<= _output_get 0)
    (Audio|PlaySound2D "/Game/Sounds/ExplosionShortCue.ExplosionShortCue")
    (Effects|SpawnEmitteratLocation "/Game/Geometry/Particles/Explosion.Explosion" _returnvalue)
    (Actor|DestroyActor)
    (else
      (Audio|PlaySound2D "/Game/Sounds/Laser.Laser")
      (Effects|SpawnEmitteratLocation "/Game/StarterContent/Particles/P_ExplosionLight.P_ExplosionLight" _returnvalue))))